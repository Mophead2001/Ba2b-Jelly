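; BP_CustomGrassPlacer is a level tool that scatters cross-shaped grass meshes over the surfaces beneath a rectangular area.
; Its construction script picks X/Y offsets from the actor root using two random streams, then line-traces vertically on Visibility, skipping excluded actors.
; Trace locations become unrotated, unit-scale transforms, without checking for a hit, and are added to a HISM in one batch.
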(fn `UserConstructionScript`
  (locals (`Root Position` :type "Vector Structure" :default (0.0 0.0 0.0)) (`Cast X` :type "Float (single-precision)" :default 0.0) (`Cast Y` :type "Float (single-precision)" :default 0.0) (`Cast Vector` :type "Vector Structure") (`Transform Array` :type "Array of Transform Structure"))
  (bind _z_ray_range (`self.Z Ray Range`))
  (`|ExecutionSequence`
    (:`then_0`
      (`StaticMeshComponent.SetStaticMesh` (`self.HISM`) "/Game/Assets/DevAssets/Grass_CrossShape.Grass_CrossShape")
      (set `local.Root Position` (`SceneComponent.K2_GetComponentLocation` (`self.DefaultSceneRoot`))))
    (:`then_1`
      (for _ (range (+ (- (`self.GrassCount`) 0) 1))
        (set `local.Cast X` (* (`KismetMathLibrary.RandomFloatFromStream` (`self.Random X`)) (`self.Range X`)))
        (set `local.Cast Y` (* (`KismetMathLibrary.RandomFloatFromStream` (`self.Random Y`)) (`self.Range Y`)))
        (bind _output_get (set `local.Cast Vector` (+ (`KismetMathLibrary.MakeVector` (`local.Cast X`) (`local.Cast Y`)) (`local.Root Position`))))
        (bind _outhit (`KismetSystemLibrary.LineTraceSingle` (+ _output_get (`KismetMathLibrary.MakeVector` 0.0 0.0 _z_ray_range)) (+ _output_get (`KismetMathLibrary.MakeVector` 0.0 0.0 (* _z_ray_range -1.0))) "TraceTypeQuery1" false (`self.Excluded Actors`)))
        (`KismetArrayLibrary.Array_Add` (`local.Transform Array`) (`KismetMathLibrary.MakeTransform` (`.Location` (`GameplayStatics.BreakHitResult` _outhit)))))
      (`InstancedStaticMeshComponent.AddInstances` (`self.HISM`) (`local.Transform Array`) false true))))