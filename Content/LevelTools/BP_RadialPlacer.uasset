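; Level tool actor that scatters copies of a mesh, such as trees, over the ground within a radius.
; The construction script picks seeded random radius and angle pairs, clustering instances toward the center, and line traces vertically at each point.
; Hit locations, without a hit check, become transforms scaled by a curve over normalized radius times a multiplier.
; All transforms are added to one instanced static mesh component in world space.
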(fn `UserConstructionScript`
  (locals (RootX :type "Float (double-precision)") (RootY :type "Float (double-precision)") (RootZ :type "Float (double-precision)") (RandRadius :type "Float (double-precision)") (RandTheta :type "Float (double-precision)") (RandVector :type "Vector Structure") (TransformArray :type "Array of Transform Structure"))
  (bind _zrayrange (`self.ZRayRange`))
  (bind _rootz (`local.RootZ`))
  (bind (_returnvalue_x _returnvalue_y _returnvalue_z) (`KismetMathLibrary.BreakVector` (`SceneComponent.K2_GetComponentLocation` (`self.DefaultSceneRoot`))))
  (bind (_relativerotation_roll _relativerotation_pitch _relativerotation_yaw) (`KismetMathLibrary.BreakRotator` (`SceneComponent.RelativeRotation` (`self.DefaultSceneRoot`))))
  (bind _returnvalue (* (`CurveFloat.GetFloatValue` (`self.Radius-Scale Curve`) (/ (`local.RandRadius`) (`self.Radius`))) (`self.Scale Multiplier`)))
  (`StaticMeshComponent.SetStaticMesh` (`self.ISM`) (`self.Mesh`))
  (set `local.RootX` _returnvalue_x)
  (set `local.RootY` _returnvalue_y)
  (set `local.RootZ` _returnvalue_z)
  (for _ (range (+ (`self.Tree Count`) 1))
    (set `local.RandRadius` (`KismetMathLibrary.RandomFloatInRangeFromStream` 0.0 (`self.Radius`) (`self.Radius Seed`)))
    (set `local.RandTheta` (`KismetMathLibrary.RandomFloatInRangeFromStream` 0.0 360.0 (`self.Theta Seed`)))
    (bind _output_get (set `local.RandVector` (`KismetMathLibrary.MakeVector` (`local.RandRadius`))))
    (bind _output_get_2 (set `local.RandVector` (`KismetMathLibrary.GreaterGreater_VectorRotator` _output_get (`KismetMathLibrary.MakeRotator` 0.0 0.0 (+ (`local.RandTheta`) _relativerotation_yaw)))))
    (bind _returnvalue_2 (+ (.x _output_get_2) (`local.RootX`)))
    (bind _returnvalue_3 (+ (.y _output_get_2) (`local.RootY`)))
    (bind _outhit (`KismetSystemLibrary.LineTraceSingle` :`Start` (`KismetMathLibrary.MakeVector` _returnvalue_2 _returnvalue_3 (+ _rootz _zrayrange)) :`End` (`KismetMathLibrary.MakeVector` _returnvalue_2 _returnvalue_3 (- _rootz _zrayrange)) :`TraceChannel` "TraceTypeQuery1" :`DrawDebugType` "ForOneFrame"))
    (`KismetArrayLibrary.Array_AddUnique` (`local.TransformArray`) (`KismetMathLibrary.MakeTransform` (`.Location` (`GameplayStatics.BreakHitResult` _outhit)) (`self.Rotation`) (`KismetMathLibrary.MakeVector` _returnvalue _returnvalue _returnvalue))))
  (`InstancedStaticMeshComponent.AddInstances` (`self.ISM`) (`local.TransformArray`) false true))