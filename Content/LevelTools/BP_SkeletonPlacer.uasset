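; BP_SkeletonPlacer is a level tool that builds a skeleton along a spline.
; The construction script adds head and end meshes at the spline's two ends.
; It fills the span between the cutoffs with mirrored pairs of instanced ribs, angled by a splay factor and scale-interpolated along the length.
; Helper functions insert a spline point near the end or remove the last one; the event graph is unused.
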(fn `Add Spline Point On End`
  (bind _spline (`self.Spline`))
  (bind _returnvalue (- (`SplineComponent.GetNumberOfSplinePoints` _spline) 1))
  (`SplineComponent.AddSplinePointAtIndex` _spline (+ (`SplineComponent.GetLocationAtSplinePoint` _spline _returnvalue "Local") (`self.New Point Offset`)) _returnvalue "Local" true))

(fn `Remove Spline Point From End`
  (bind _spline (`self.Spline`))
  (`SplineComponent.RemoveSplinePoint` _spline (- (`SplineComponent.GetNumberOfSplinePoints` _spline) 1) true))

(fn `UserConstructionScript`
  (bind _splay_factor (`self.Splay Factor`))
  (bind _spline (`self.Spline`))
  (bind _returnvalue (`SplineComponent.GetSplineLength` (`self.Spline`)))
  (`|ExecutionSequence`
    (:`then_0`
      (`StaticMeshComponent.SetStaticMesh` (`self.InstancedStaticMesh`) (`self.RibMesh`)))
    (:`then_1`
      ;[1 1 1] Place Head
      (bind _returnvalue_2 (`AddComponent|NODE_AddStaticMeshComponent-2` :`RelativeTransform` (`SplineComponent.GetTransformAtDistanceAlongSpline` (`self.Spline`) 0.0 "Local" false)))
      (`StaticMeshComponent.SetStaticMesh` _returnvalue_2 (`self.HeadMesh`)))
    (:`then_2`
      ;[1 1 1] Place End
      (bind _returnvalue_3 (`AddComponent|NODE_AddStaticMeshComponent-0` :`RelativeTransform` (`SplineComponent.GetTransformAtDistanceAlongSpline` _spline (`SplineComponent.GetSplineLength` _spline) "Local" false)))
      (`StaticMeshComponent.SetStaticMesh` _returnvalue_3 (`self.EndMesh`)))
    (:`then_3`
      (for _index (range (`self.RibCount`))
        (bind _returnvalue_4 (/ _index (- (`self.RibCount`) 1)))
        (bind (_returnvalue_location _returnvalue_rotation) (`KismetMathLibrary.BreakTransform` (`SplineComponent.GetTransformAtDistanceAlongSpline` (`self.Spline`) (`KismetMathLibrary.Lerp` (* _returnvalue (`self.HeadCutoff`)) (* _returnvalue (`self.EndCutoff`)) _returnvalue_4) "Local" false)))
        (bind _returnvalue_5 (* (2.0 2.0 2.0) (`KismetMathLibrary.VLerp` (* (1.0 1.0 1.0) (`self.Scale Lerp Min`)) (* (1.0 1.0 1.0) (`self.Scale Lerp Max`)) _returnvalue_4)))
        (`InstancedStaticMeshComponent.AddInstance` (`self.InstancedStaticMesh`) (`KismetMathLibrary.MakeTransform` _returnvalue_location (`KismetMathLibrary.ComposeRotators` (`KismetMathLibrary.MakeRotator` 0.0 _splay_factor -90.0) _returnvalue_rotation) _returnvalue_5) false)
        (`InstancedStaticMeshComponent.AddInstance` (`self.InstancedStaticMesh`) (`KismetMathLibrary.MakeTransform` _returnvalue_location (`KismetMathLibrary.ComposeRotators` (`KismetMathLibrary.MakeRotator` 0.0 _splay_factor 90.0) _returnvalue_rotation) _returnvalue_5) false)))))