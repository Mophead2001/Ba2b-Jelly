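; BPC_PlayerController is a player controller that turns input axes into swimming and camera commands for the player's BP_Diver pawn.
; BeginPlay casts and caches the pawn as DiverPawn.
; Both camera axes share one CameraMovement call, and vertical input drives SwimZAxis directly.
; Forward and sideways input share one SwimXYPlane call, with values normalized to constrain their range.
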(event `self.ReceiveBeginPlay`
  (bind _asbp_diver (cast `/Game/Blueprints/BP_Diver` (`GameplayStatics.GetPlayerPawn` 0)))
  (set `self.Diver Pawn` _asbp_diver))

(event `InputAxis|Camera_X`
  (params (AxisValue :type "Float (single-precision)"))
  (`/Game/Blueprints/BP_Diver.CameraMovement` (`self.Diver Pawn`) AxisValue (stale `InputAxis|Camera_Y` AxisValue) :!label _label))

(event `InputAxis|Camera_Y`
  (params (AxisValue :type "Float (single-precision)"))
  (goto _label))

(event `InputAxis|Swim_Up`
  (params (AxisValue :type "Float (single-precision)"))
  ;[1 1 1] Swimming Motion
  (`/Game/Blueprints/BP_Diver.Swim Z Axis` (`self.Diver Pawn`) AxisValue))

(event `InputAxis|SwimForward`
  (params (AxisValue :type "Float (single-precision)"))
  ;[1 1 1] Swimming Motion
  (bind (_returnvalue_x _returnvalue_y) (`KismetMathLibrary.BreakVector` (`KismetMathLibrary.Normal` (`KismetMathLibrary.MakeVector` AxisValue (stale `InputAxis|SwimSideways` AxisValue)))))
  (`/Game/Blueprints/BP_Diver.Swim XY Plane` (`self.Diver Pawn`) _returnvalue_x _returnvalue_y :!label _label_2))

(event `InputAxis|SwimSideways`
  (params (AxisValue :type "Float (single-precision)"))
  ;[1 1 1] Swimming Motion
  (goto _label_2))

(fn `UserConstructionScript`)