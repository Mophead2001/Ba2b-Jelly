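; Player diver pawn that swims without gravity and toggles a photo mode with viewfinder to photograph fish.
; Right click in photo mode captures the scene to a new render target, shown in a result widget and stored for the album.
; TraceLineArray scores shots by sweeping a line-trace grid across the view, bounding each fish hit, then applying rarity, rule-of-thirds and subject variety/count bonuses.
; Album scores are stored as zero.
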(event `self.ReceiveBeginPlay`
  (`PrimitiveComponent.SetEnableGravity` (`self.CapsuleComponent`) false))

(event `CameraMovement`
  (params (XAxis :type "Float (double-precision)") (YAxis :type "Float (double-precision)"))
  (bind (_relativerotation_roll _relativerotation_pitch _relativerotation_yaw) (`KismetMathLibrary.BreakRotator` (`SceneComponent.RelativeRotation` (`self.SpringArm`))))
  ;[1 1 1] Camera Motion
  (`SceneComponent.K2_SetRelativeRotation` (`self.SpringArm`) (`KismetMathLibrary.MakeRotator` 0.0 (`KismetMathLibrary.FClamp` (+ YAxis _relativerotation_pitch) (`self.[PARAM]CamAngleMin`) (`self.[PARAM]CamAngleMax`)) (+ XAxis _relativerotation_yaw)) false false))

(event `Swim Z Axis`
  (params (AxisValue :type "Float (double-precision)"))
  ;[1 1 1] Movement Controls
  (`self.Movement PermissionCheck`
    (:`OutputPin`
      (`self.AddMovementInput` (0.0 0.0 1.0) (* AxisValue 0.5)))))

(event `Swim XY Plane`
  (params (ForwardAxis :type "Float (double-precision)") (RightAxis :type "Float (double-precision)"))
  (bind _defaultcam (`self.DefaultCam`))
  ;[1 1 1] Movement Controls
  (`self.Movement PermissionCheck`
    (:`OutputPin`
      (`self.AddMovementInput` (+ (* ForwardAxis (`SceneComponent.GetForwardVector` _defaultcam)) (* RightAxis (`SceneComponent.GetRightVector` _defaultcam)))))))

(event `Toggle Cam Modes`
  ;[1 1 1] Toggle Between Modes
  (switch `/Game/DataStructures/E_DiverState` (`self.State Enum`)
    (:`NewEnumerator0`
      (`ActorComponent.SetActive` (`self.PhotoCam`) true false :!label _label)
      (`ActorComponent.SetActive` (`self.DefaultCam`) false false)
      (set `self.State Enum` "NewEnumerator2")
      (bind _returnvalue (`|CreateWidget` "/Game/Blueprints/WBP_CameraViewFinder.WBP_CameraViewFinder_C" null (`SceneCaptureComponent2D.FOVAngle` (`self.SceneCapComponent`))))
      (bind _output_get (set `self.Viewfinder` _returnvalue))
      (`UserWidget.AddToViewport` _output_get 0))
    (:`NewEnumerator1`
      (goto _label))
    (:`NewEnumerator2`
      (`ActorComponent.SetActive` (`self.DefaultCam`) true false)
      (`ActorComponent.SetActive` (`self.PhotoCam`) false false)
      (set `self.State Enum` "NewEnumerator0")
      (`Widget.RemoveFromParent` (`self.Viewfinder`)))))

(event `Key|RightMouseButton`
  (params (Key :type "Key Structure"))
  ;[1 1 1] Photo Taking Function
  (:`Pressed`
    (switch `/Game/DataStructures/E_DiverState` (`self.State Enum`)
      (:`NewEnumerator2`
        (bind _returnvalue (`KismetRenderingLibrary.CreateRenderTarget2D` (`self.RenderXSize`) (`self.RenderYSize`)))
        (bind _output_get (set `SceneCaptureComponent2D.TextureTarget` _returnvalue (`self.SceneCapComponent`)))
        (`SceneCaptureComponent2D.CaptureScene` (`self.SceneCapComponent`))
        ;;[1 0.06447 0.3582] Line Tracer Detection
        (bind (_score _modifier_tag) (`self.TraceLineArray` (`self.TracerXResolution`) (`self.TracerYResolution`) (/ (`self.RenderYSize`) (`self.RenderXSize`))))
        (bind _returnvalue_2 (`|CreateWidget` "/Game/Blueprints/WBP_PhotoResult.WBP_PhotoResult_C" (`GameplayStatics.GetPlayerController` 0) _output_get (`self.RenderXSize`) (`self.RenderYSize`) _score _modifier_tag))
        (`UserWidget.AddToViewport` _returnvalue_2 0)
        (`KismetArrayLibrary.Array_Add` (`self.Render Targets`) _output_get)
        (`KismetArrayLibrary.Array_Add` (`self.Photo Scores`))))))

(event `Key|RightShift`
  (params (Key :type "Key Structure"))
  (:`Pressed`
    (`/Engine/EditorBlueprintResources/StandardMacros.FlipFlop`
      (:`A`
        (bind _returnvalue (`|CreateWidget` "/Game/Blueprints/WBP_PhotoAlbum.WBP_PhotoAlbum_C" null (`self.Photo Scores`) (`self.Render Targets`)))
        (`UserWidget.AddToViewport` _returnvalue 0))
      (:`B`
        (`Widget.RemoveFromParent` _returnvalue)))))

(fn `TraceLineArray`
  (params (`X Resolution` :type Integer :default 5) (`Y Resolution` :type Integer :default 5) (`Aspect Ratio` :type "Float (double-precision)"))
  (returns (Score :type "Float (double-precision)") (`Modifier Tag` :type "/Game/DataStructures/E_ScoreModifiers Enum"))
  (locals (`Forward Vector` :type "Vector Structure") (`Right Vector` :type "Vector Structure" :default (0.0 0.0 0.0)) (`Up Vector` :type "Vector Structure" :default (0.0 0.0 0.0)) (Location :type "Vector Structure") (`Vertical Angle Offset` :type "Float (double-precision)") (`Horizontal Angle Offset` :type "Float (double-precision)") (TempVector1 :type "Vector Structure") (CastVectorArray :type "Vector Structure") (TempVector2 :type "Vector Structure") (TracerTrigger :type "Float (double-precision)") (`Vertical Fraction` :type "Float (double-precision)") (`Right Fraction` :type "Float (double-precision)") (`Hit Data` :type "/Game/DataStructures/Struct_PhotoHitData Structure") (`Input PhotoData` :type "/Game/DataStructures/Struct_PhotoHitData Structure"))
  (bind _scenecapcomponent (`self.SceneCapComponent`))
  (bind _vertical_fraction (`local.Vertical Fraction`))
  (bind _right_fraction (`local.Right Fraction`))
  (bind _location (`local.Location`))
  (bind _returnvalue (/ (`self.Vertical Field of View`) 2.0))
  (bind _returnvalue_2 (/ (`self.Horizontal Field of View`) 2.0))
  (set `self.Horizontal Field of View` (`SceneCaptureComponent2D.FOVAngle` (`self.SceneCapComponent`)))
  (set `self.Vertical Field of View` (* `Aspect Ratio` (`self.Horizontal Field of View`)))
  (set `local.Forward Vector` (`SceneComponent.GetForwardVector` _scenecapcomponent))
  (set `local.Right Vector` (`SceneComponent.GetRightVector` _scenecapcomponent))
  (set `local.Up Vector` (`SceneComponent.GetUpVector` _scenecapcomponent))
  (set `local.Location` (`SceneComponent.K2_GetComponentLocation` _scenecapcomponent))
  (set `local.Vertical Angle Offset` (/ (`self.Horizontal Field of View`) `Y Resolution`))
  (set `local.Horizontal Angle Offset` (/ (`self.Horizontal Field of View`) `X Resolution`))
  (`|ExecutionSequence`
    (:`then_0`
      (`KismetArrayLibrary.Array_Clear` (`self.Photo Hit Data`))
      (`KismetArrayLibrary.Array_Clear` (`self.Fish Object Ref`))
      (`KismetArrayLibrary.Array_Clear` (`self.Hit Name Arrays`))
      (`KismetArrayLibrary.Array_Clear` (`self.Fish Class Ref`)))
    (:`then_1`
      (set `local.TracerTrigger` 0.0)
      (for _index (range `Y Resolution`)
        (bind _output_get (set `local.TempVector1` (`local.Forward Vector`)))
        (bind _returnvalue_3 (/ (`KismetMathLibrary.Conv_IntToDouble` _index) (- (`self.TracerYResolution`) 1)))
        (set `local.Vertical Fraction` _returnvalue_3)
        (set `local.TempVector1` (`KismetMathLibrary.RotateAngleAxis` _output_get (`KismetMathLibrary.Lerp` (- 0.0 _returnvalue) _returnvalue _returnvalue_3) (`local.Right Vector`)))
        (for _index_2 (range `X Resolution`)
          (bind _returnvalue_4 (/ (`KismetMathLibrary.Conv_IntToDouble` _index_2) (- (`self.TracerXResolution`) 1)))
          (set `local.Right Fraction` _returnvalue_4)
          (set `local.TempVector2` (`KismetMathLibrary.RotateAngleAxis` (`local.TempVector1`) (`KismetMathLibrary.Lerp` (- 0.0 _returnvalue_2) _returnvalue_2 _returnvalue_4) (`local.Up Vector`)))
          (bind (_outhit _returnvalue_5) (`KismetSystemLibrary.LineTraceSingleForObjects` :`Start` _location :`End` (+ _location (* (`local.TempVector2`) (`self.LineTraceDistance`))) :`ObjectTypes` (`self.Object Types`) :`bTraceComplex` true :`TraceColor` (struct :`R` 1.0 :`G` 0.343419 :`B` 0.871042 :`A` 1.0) :`TraceHitColor` (struct :`R` 0.512023 :`G` 1.0 :`B` 0.163483 :`A` 1.0) :`DrawTime` 15.0))
          (if _returnvalue_5
            (bind _asbp_fish_parent (cast `/Game/Blueprints/BP_Fish_Parent` (`.HitActor` (`GameplayStatics.BreakHitResult` _outhit))))
            (bind _returnvalue_6 (`KismetArrayLibrary.Array_Find` (`self.Fish Object Ref`) _asbp_fish_parent))
            (if (== _returnvalue_6 -1)
              (`KismetArrayLibrary.Array_Add` (`self.Fish Object Ref`) _asbp_fish_parent)
              (`KismetArrayLibrary.Array_Add` (`self.Photo Hit Data`) (make `/Game/DataStructures/Struct_PhotoHitData` _right_fraction _vertical_fraction _right_fraction _vertical_fraction (`/Game/Blueprints/BP_Fish_Parent.Rarity Score` _asbp_fish_parent) _asbp_fish_parent))
              (`KismetArrayLibrary.Array_AddUnique` (`self.Fish Class Ref`) (`GameplayStatics.GetObjectClass` _asbp_fish_parent))
              (else
                (bind (_output_x_0 _output_y_0 _output_x_1 _output_y_1 _output_score _output_membervar) (break `/Game/DataStructures/Struct_PhotoHitData` (`|GetArrayItem` (`self.Photo Hit Data`) _returnvalue_6)))
                (if (> (`local.Right Fraction`) _output_x_1)
                  (`KismetArrayLibrary.Array_Set` (`self.Photo Hit Data`) _returnvalue_6 (make `/Game/DataStructures/Struct_PhotoHitData` _output_x_0 _output_y_0 (`local.Right Fraction`) _output_x_1 _output_score _output_membervar))
                  (elif (> (`local.Vertical Fraction`) _output_y_1)
                    (`KismetArrayLibrary.Array_Set` (`self.Photo Hit Data`) _returnvalue_6 (make `/Game/DataStructures/Struct_PhotoHitData` _output_x_0 _output_y_0 _output_x_1 (`local.Vertical Fraction`) _output_score _output_membervar)))))))))
      (`|ExecutionSequence`
        (:`then_0`
          (set `self.Score` 0.0)
          (for _array_element (`self.Photo Hit Data`)
            (set `self.Score` (+ (`self.Score`) (`.Score_22_B8DB26DD41133334EE6395A0F6C83FFE` (break `/Game/DataStructures/Struct_PhotoHitData` _array_element))))
            (if (and (`self.Contains Rule of Thirds Marker` (break `/Game/DataStructures/Struct_PhotoHitData` _array_element) (`.X_1_18_996BB7334BA1181AA33762A212879747` (break `/Game/DataStructures/Struct_PhotoHitData` _array_element))) (`self.Contains Rule of Thirds Marker` (`.Y_0_15_001E5D144B3789C132B63092E70C0BB3` (break `/Game/DataStructures/Struct_PhotoHitData` _array_element)) (`.Y_1_20_CA2FA3C94FC9095198384D9E2A50B593` (break `/Game/DataStructures/Struct_PhotoHitData` _array_element))))
              (`KismetSystemLibrary.PrintString` "Good")
              (set `self.Score` (* (`self.Well Composed Multiplier`) (`self.Score`)))
              (else
                (`KismetSystemLibrary.PrintString` "Bad")))))
        (:`then_1`
          (if (>= (`KismetArrayLibrary.Array_Length` (`self.Fish Class Ref`)) 3)
            (bind _output_get_2 (set `self.Score` (* (`self.Score`) (`self.Diverse Subjects`))))
            (return _output_get_2 "NewEnumerator2")
            (elif (>= (`KismetArrayLibrary.Array_Length` (`self.Fish Object Ref`)) 3)
              (bind _output_get_3 (set `self.Score` (* (`self.Score`) (`self.Multiple Subjects`))))
              (return _output_get_3 "NewEnumerator1")
              (else
                (return (`self.Score`) "NewEnumerator0")))))))))

(fn `UserConstructionScript`)