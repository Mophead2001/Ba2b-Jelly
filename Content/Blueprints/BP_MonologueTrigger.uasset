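; BP_MonologueTrigger is a placeable box trigger that passes its TextLine to BP_Diver's MonologueTrigger when overlapped.
; The overlap fires through a DoOnce placed before the diver cast, so the first overlapping actor of any type uses up the trigger.
; The construction script shows the line on a TextRender and scales the box from BoxDimensions.
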(event `self.Box.OnComponentBeginOverlap`
  (params (OverlappedComponent :type "PrimitiveComponent Object Reference") (OtherActor :type "Actor Object Reference") (OtherComp :type "PrimitiveComponent Object Reference") (OtherBodyIndex :type Integer) (bFromSweep :type Boolean) (SweepResult :type "HitResult Structure (by ref)"))
  (`/Engine/EditorBlueprintResources/StandardMacros.DoOnce` false
    (:`Completed`
      (bind _asbp_diver (cast `/Game/Blueprints/BP_Diver` OtherActor))
      (`/Game/Blueprints/BP_Diver.Monologue Trigger` _asbp_diver (`self.Text Line`)))))

(event `self.Box.OnComponentEndOverlap`
  (params (OverlappedComponent :type "PrimitiveComponent Object Reference") (OtherActor :type "Actor Object Reference") (OtherComp :type "PrimitiveComponent Object Reference") (OtherBodyIndex :type Integer)))

(fn `UserConstructionScript`
  (`TextRenderComponent.K2_SetText` (`self.TextRender`) (`self.Text Line`))
  (`SceneComponent.SetRelativeScale3D` (`self.Box`) (`self.BoxDimensions`)))