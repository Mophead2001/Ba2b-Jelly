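; Parent Blueprint for fish that swim repeatedly along a spline, with species looks and rarity data drawn from a data table.
; On BeginPlay a timeline starts at a random time, moves and rotates the mesh by spline distance, and restarts from zero when finished.
; FetchAndConstruct loads a named row's rarity, species, mesh and material, then applies the visuals; nothing here calls it.
; A similar lookup in the event graph is disconnected.
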(event `self.ReceiveBeginPlay`
  (`self.StartMotion` (* (`KismetMathLibrary.RandomFloat`) 20.0)))

(event `StartMotion`
  (params (StartValue :type "Float (double-precision)"))
  (bind _spline (`self.Spline`))
  (bind _static_mesh_component (`self.Static Mesh Component`))
  (`|ExecutionSequence`
    (:`then_0`
      (bind (_direction _newtrack_0) (`Timeline|MoveTimeline` :`NewTime` StartValue :!via `SetNewTime` :!label _label)
        (:`Update`
          (bind (_returnvalue_location _returnvalue_rotation) (`KismetMathLibrary.BreakTransform` (`SplineComponent.GetTransformAtDistanceAlongSpline` _spline (* _newtrack_0 (`SplineComponent.GetSplineLength` _spline)) "Local" false)))
          (`SceneComponent.K2_SetRelativeTransform` _static_mesh_component (`KismetMathLibrary.MakeTransform` _returnvalue_location _returnvalue_rotation (`SceneComponent.RelativeScale3D` _static_mesh_component)) false false))
        (:`Finished`
          (`self.StartMotion` 0.0))))
    (:`then_1`
      (goto _label))))

(fn `Fetch and Construct`
  (params (NAME :type Name))
  (bind _returnvalue (`|GetDataTableRow` (`self.Data Table`) NAME)
    (:`then`
      (bind (_rarity_score _species_name _static_mesh _mesh_material) (break `/Game/DataStructures/Struct_FishData` _returnvalue))
      (set `self.Rarity Score` _rarity_score)
      (set `self.Species Name` _species_name)
      (set `self.Static Mesh` _static_mesh)
      (set `self.Mesh Material` _mesh_material)
      (`StaticMeshComponent.SetStaticMesh` (`self.Static Mesh Component`) (`self.Static Mesh`))
      (`PrimitiveComponent.SetMaterial` (`self.Static Mesh Component`) 0 (`self.Mesh Material`)))))

(fn `UserConstructionScript`)