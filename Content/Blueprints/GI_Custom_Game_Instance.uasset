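; Custom game instance that holds an array of fish species data for a game with photographing and discovery entries.
; ConstructDataFunct clears the array, rebuilds it from every FishDataTable row (rarity, name, mesh, material, photo state, journal text) and returns it.
; FetchFishData does the same without returning it, but takes row names from a column lookup with property None.
; The ConstructData event is an empty stub.
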(event `Construct Data`)

(fn `ConstructDataFunct`
  (returns (NewParam :type "Array of /Game/DataStructures/Struct_FishData Structure"))
  (bind _fishdatatable (`self.FishDataTable`))
  (`KismetArrayLibrary.Array_Clear` (`self.Fish Data Array`))
  (bind _outrownames (`DataTableFunctionLibrary.GetDataTableRowNames` _fishdatatable))
  (for _array_element _outrownames
    (bind _returnvalue (`|GetDataTableRow` _fishdatatable _array_element)
      (:`then`
        (bind (_rarity_score _species_name _static_mesh _mesh_material _is_photographed _render_photo _unseen_entry _discovered_entry) (break `/Game/DataStructures/Struct_FishData` _returnvalue))
        (`KismetArrayLibrary.Array_Add` (`self.Fish Data Array`) (make `/Game/DataStructures/Struct_FishData` _rarity_score _species_name _static_mesh _mesh_material _is_photographed _render_photo _unseen_entry _discovered_entry)))))
  (return (`self.Fish Data Array`)))

(fn `Fetch FishData`
  (bind _fishdatatable (`self.FishDataTable`))
  (`KismetArrayLibrary.Array_Clear` (`self.Fish Data Array`))
  (bind _returnvalue (`DataTableFunctionLibrary.GetDataTableColumnAsString` _fishdatatable))
  (for _array_element _returnvalue
    (bind _returnvalue_2 (`|GetDataTableRow` _fishdatatable (`KismetStringLibrary.Conv_StringToName` _array_element))
      (:`then`
        (bind (_rarity_score _species_name _static_mesh _mesh_material _is_photographed _render_photo _unseen_entry _discovered_entry) (break `/Game/DataStructures/Struct_FishData` _returnvalue_2))
        (`KismetArrayLibrary.Array_Add` (`self.Fish Data Array`) (make `/Game/DataStructures/Struct_FishData` _rarity_score _species_name _static_mesh _mesh_material _is_photographed _render_photo _unseen_entry _discovered_entry))))))